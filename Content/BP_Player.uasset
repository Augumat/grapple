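; Player actor with custom velocity-based movement: drifting, cooldown-limited dashing and grappling, plus a respawn-style KillPlayer teleport.
; Each Tick, UpdatePhysics reads BP_PlayerInputReceiver for heading and button states, then sums drift, dash and grapple offsets into Velocity.
; Velocity persists and moves the actor by a swept per-frame XY offset, unscaled by delta time, until a hit zeroes it.
; FireGrapple spawns BP_Grapple_Projectile; while grappled, holding pulls toward GrappleLocation.
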(event OnComponentHit(Body)
  (params (HitComponent :type Primitive%20Component%20Object%20Reference) (OtherActor :type Actor%20Object%20Reference) (OtherComp :type Primitive%20Component%20Object%20Reference) (NormalImpulse :type Vector :default "0, 0, 0") (Hit :type Hit%20Result%20Structure%20%28by%20ref%29))
  ;[1 1 1] Colliding with either a wall, player, or blastzone
  (Variables|Default|SetVelocity "0, 0, 0"))

(event OnComponentBeginOverlap(Body)
  (params (OverlappedComponent :type Primitive%20Component%20Object%20Reference) (OtherActor :type Actor%20Object%20Reference) (OtherComp :type Primitive%20Component%20Object%20Reference) (OtherBodyIndex :type Integer) (bFromSweep :type Boolean) (SweepResult :type Hit%20Result%20Structure%20%28by%20ref%29)))

(event EventTick
  (params (DeltaSeconds :type Float%20%28single-precision%29))
  (CallFunction|UpdatePhysics DeltaSeconds))

(fn ConstructionScript)

(fn UpdatePhysics
  (params (dt :type Float%20%28single-precision%29))
  (bind _cable (Variables|Default|GetCable))
  (LocalVariables|SetTimestep dt)
  (bind _returnvalue (Actor|GetActorOfClass "/Game/BP_PlayerInputReceiver.BP_PlayerInputReceiver_C"))
  (LocalVariables|SetInput _returnvalue)
  (Utilities|FlowControl|Sequence
    (:then_0
      ;[1 1 1] rotation
      (Transformation|SetActorRotation (Variables|/Game/BP_PlayerInputReceiver.BP_PlayerInputReceiver_C|GetHeadingRotator (LocalVariables|GetInput))))
    (:then_1
      ;[1 1 1] drifting
      (bind _direction_vector (CallFunction|GetTotalDriftInput (LocalVariables|GetInput)))
      (LocalVariables|SetNew%20Velocity%20Offset (* _direction_vector (Variables|Default|GetDrift%20Power))))
    (:then_2
      ;[1 1 1] dashing
      (if (> (Variables|Default|GetFrames%20Since%20Last%20Dash2) (Variables|Default|GetDash%20CD%20%28frames%29))
        ;;[1 1 0] Verifies a direction is pressed before dashing
        (bind _direction_vector_2 (CallFunction|GetTotalDriftInput (LocalVariables|GetInput)))
        (if (> (Math|Vector|VectorLength _direction_vector_2) 0.0)
          (switch Utilities|FlowControl|Switch|SwitchonButtonInputState (Utilities|Array|Get(acopy) (Variables|/Game/BP_PlayerInputReceiver.BP_PlayerInputReceiver_C|GetCurrentFrameInputs (LocalVariables|GetInput)) 4)
            (:NewEnumerator1
              (LocalVariables|SetNew%20Velocity%20Offset (+ (* _direction_vector_2 (Variables|Default|GetDash%20Power)) (LocalVariables|GetNew%20Velocity%20Offset)))
              (Variables|Default|SetFrames%20Since%20Last%20Dash2 0)
              (Development|PrintString "dashing?"))))))
    (:then_3
      ;[1 1 1] Grappling here
      (if (Variables|Default|GetIsGrappled)
        (switch Utilities|FlowControl|Switch|SwitchonButtonInputState (Utilities|Array|Get(acopy) (Variables|/Game/BP_PlayerInputReceiver.BP_PlayerInputReceiver_C|GetCurrentFrameInputs (LocalVariables|GetInput)) 7)
          (:NewEnumerator0
            ;;[1 0.3301 0.2999] Stop Grappling
            (Variables|Default|SetIsGrappled false)
            (Rendering|SetVisibility _cable false false))
          (:NewEnumerator2
            ;;[1 0.9573 0.2956] Go towards the object while grappled
            (bind _returnvalue_2 (CallFunction|CalculateGrappleVelocityOffset))
            (LocalVariables|SetGrappleVelocityOffset _returnvalue_2)
            (Rendering|SetVisibility _cable true false)))
        (else
          ;;[0.5403 1 0.5329] Fire Grapple if not grappled yet and button is pressed
          (switch Utilities|FlowControl|Switch|SwitchonButtonInputState (Utilities|Array|Get(acopy) (Variables|/Game/BP_PlayerInputReceiver.BP_PlayerInputReceiver_C|GetCurrentFrameInputs (LocalVariables|GetInput)) 7)
            (:NewEnumerator1
              (CallFunction|FireGrapple (Variables|/Game/BP_PlayerInputReceiver.BP_PlayerInputReceiver_C|GetHeadingRotator (LocalVariables|GetInput))))))))
    (:then_4
      ;[1 1 1] Moving the Player
      (bind _output_get (Variables|Default|SetVelocity (+ (Variables|Default|GetVelocity) (+ (LocalVariables|GetNew%20Velocity%20Offset) (LocalVariables|GetGrappleVelocityOffset)))))
      (Transformation|AddActorWorldOffset (Math|Vector|MakeVector (.X (Math|Vector|BreakVector _output_get)) (.Y (Math|Vector|BreakVector _output_get)) 0.0) true)
      (LocalVariables|SetNew%20Velocity%20Offset "0, 0, 0")
      (LocalVariables|SetGrappleVelocityOffset "0, 0, 0")
      (CallFunction|UpdateTimers))))

(fn GetTotalDriftInput
  (params (Input :type BP%20Player%20Input%20Receiver%20Object%20Reference))
  (bind _currentframeinputs (Variables|/Game/BP_PlayerInputReceiver.BP_PlayerInputReceiver_C|GetCurrentFrameInputs Input))
  ;[1 1 1] Given Input, provides X and Y values that correspond to what is being held by the player
  (Utilities|FlowControl|Sequence
    (:then_0
      (switch Utilities|FlowControl|Switch|SwitchonButtonInputState (Utilities|Array|Get(acopy) _currentframeinputs)
        (:NewEnumerator1
          _)
        (:NewEnumerator2
          _))
      (LocalVariables|Setcurr%20y -1.0))
    (:then_1
      (switch Utilities|FlowControl|Switch|SwitchonButtonInputState (Utilities|Array|Get(acopy) _currentframeinputs 1)
        (:NewEnumerator1
          _)
        (:NewEnumerator2
          _))
      (LocalVariables|Setcurr%20y (+ (LocalVariables|Getcurr%20y) 1.0)))
    (:then_2
      (switch Utilities|FlowControl|Switch|SwitchonButtonInputState (Utilities|Array|Get(acopy) _currentframeinputs 2)
        (:NewEnumerator1
          _)
        (:NewEnumerator2
          _))
      (LocalVariables|Setcurr%20x 1.0))
    (:then_3
      (switch Utilities|FlowControl|Switch|SwitchonButtonInputState (Utilities|Array|Get(acopy) _currentframeinputs 3)
        (:NewEnumerator1)
        (:NewEnumerator2
          (LocalVariables|Setcurr%20x (+ -1.0 (LocalVariables|Getcurr%20x))))))
    (:then_4
      (return (Math|Vector|Normalize (Math|Vector|MakeVector (LocalVariables|Getcurr%20x) (LocalVariables|Getcurr%20y) 0.0))))))

(fn KillPlayer
  (Transformation|SetActorLocation "0.000000, 0,300.000000" false true)
  (Variables|Default|SetIsGrappled false)
  (Rendering|SetVisibility (Variables|Default|GetCable) false false)
  (Development|PrintString "You have died" true true "(R=0.291667,G=0.015041,B=0.000000,A=1.000000)"))

(fn UpdateTimers
  ;[1 1 1] Function to update any needed timers/cooldowns (dash CD, maybe grappling CD, etc.)
  (bind _result (Math|Integer|IncrementInt (Variables|Default|GetFrames%20Since%20Last%20Dash2))
    (:%20%20
      (Variables|Default|SetFrames%20Since%20Last%20Dash2 _result))))

(fn FireGrapple
  (params (Heading :type Rotator))
  (bind _returnvalue (Game|SpawnActorfromClass "/Game/BP_Grapple_Projectile.BP_Grapple_Projectile_C" (Math|Transform|MakeTransform (+ (Transformation|GetActorLocation) (* (Math|Vector|GetForwardVector Heading) 1e+02)) Heading) "Undefined" 0 0))
  (if (Utilities|IsValid _returnvalue)
    ;[1 1 1] Tell projectile who it was fired by
    (Variables|/Game/BP_Grapple_Projectile.BP_Grapple_Projectile_C|SetPlayer _returnvalue self)))

(fn CalculateGrappleVelocityOffset
  (return (* (Math|Vector|Normalize (- (Variables|Default|GetGrappleLocation) (Transformation|GetActorLocation))) (Variables|Default|GetGrapplePower))))