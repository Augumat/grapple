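; BP_SpeedZone is a zone actor that kills BP_Player if it begins overlapping at or below SafeSpeed.
; The overlap event compares the player's velocity magnitude against that threshold before calling KillPlayer.
; Tick looks up the player and repeats the speed check to set the Cube's material, though both branches apply M_SpeedZone.
; Gradient and dynamic material nodes are left unconnected.
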(event EventTick
  (params (DeltaSeconds :type Float%20%28single-precision%29))
  (bind _returnvalue (Actor|GetActorOfClass "/Game/BP_Player.BP_Player_C"))
  (bind _asbp_player (Utilities|Casting|CastToBP_Player _returnvalue))
  (if (> (Math|Vector|VectorLength (Variables|/Game/BP_Player.BP_Player_C|GetVelocity _asbp_player)) (Variables|Default|GetSafeSpeed))
    (Rendering|Material|SetMaterial (Variables|Default|GetCube) 0 "/Game/Materials/M_SpeedZone.M_SpeedZone")
    (else
      (Rendering|Material|SetMaterial (Variables|Default|GetCube) 0 "/Game/Materials/M_SpeedZone.M_SpeedZone"))))

(event Collision|EventActorBeginOverlap
  (params (OtherActor :type Actor%20Object%20Reference))
  (bind _asbp_player (Utilities|Casting|CastToBP_Player OtherActor))
  (if (not (> (Math|Vector|VectorLength (Variables|/Game/BP_Player.BP_Player_C|GetVelocity _asbp_player)) (Variables|Default|GetSafeSpeed)))
    (Default|KillPlayer _asbp_player)))

(fn ConstructionScript)