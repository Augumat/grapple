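; Game mode for testing movement, which sets up a fixed match camera on BeginPlay.
; It spawns BP_MatchCamera high above the world origin, stores it and makes it player 0's view target.
; It then looks up a PlayerStart, but the nodes that would spawn and store BP_PlayerInputReceiver and BP_Player at its transform are disconnected and never run.
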(event EventBeginPlay
  ;[0.6 0.6 1] Camera Setup
  (bind _returnvalue (Game|SpawnActorfromClass "/Game/BP_MatchCamera.BP_MatchCamera_C" (Math|Transform|MakeTransform "0, 0,2000.000000" "-90.000000,0.000000, 0") "Undefined" 0 0))
  (bind _output_get (Variables|Default|SetMatchCamera _returnvalue))
  (Game|Player|SetViewTargetwithBlend (Game|GetPlayerController 0) _output_get 0.0 "VTBlend_Linear" 0.0 false)
  ;[1 0.6 0.6] Player Setup
  (bind _returnvalue_2 (Actor|GetActorOfClass "/Script/Engine.PlayerStart")))

(fn ConstructionScript)