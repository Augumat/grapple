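; BP_BackWall is a wall display that shows a timer and a list of recorded lap splits.
; LapTimer receives new timer text and, when flagged as a lap, first saves the previous text to an array of split entries.
; Every Tick writes the current text to TimerDisplay and rebuilds SplitDisplay by concatenating all saved entries, then clears the string buffer.
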(event EventBeginPlay)

(event Collision|EventActorBeginOverlap
  (params (OtherActor :type Actor%20Object%20Reference)))

(event EventTick
  (params (DeltaSeconds :type Float%20%28single-precision%29))
  (Rendering|Components|TextRender|SetText (Variables|Default|GetTimerDisplay) (Utilities|Text|ToText(String) (Variables|Default|GetTimerDisplayText)))
  (for _array_element (Variables|Default|GetTimerDisplayLines)
    (Variables|Default|SetStringBuilder (Utilities|String|Append (Variables|Default|GetStringBuilder) " 
" _array_element)))
  (Rendering|Components|TextRender|SetText (Variables|Default|GetSplitDisplay) (Utilities|Text|ToText(String) (Variables|Default|GetStringBuilder)))
  (Variables|Default|SetStringBuilder ""))

(fn ConstructionScript)

(fn LapTimer
  (params (NewParam :type String) (Lap :type Boolean))
  (if Lap
    (Utilities|Array|Add (Variables|Default|GetTimerDisplayLines) (Variables|Default|GetTimerDisplayText)))
  (Variables|Default|SetTimerDisplayText NewParam))