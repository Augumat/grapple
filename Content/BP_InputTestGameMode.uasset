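; BP_InputTestGameMode is a game mode for testing local multiplayer menu input through the WM Input Manager.
; On BeginPlay it adds the WM_InputManagerSmartMenu widget to the viewport, starts the input manager's UMG mode with zero players, then creates four local players.
; Each Tick it passes the current player count to the input manager.
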(event EventBeginPlay
  (bind _returnvalue (Class|WMControllerFunctionLib|GetWMInputManager))
  (Utilities|FlowControl|Sequence
    (:then_0
      (bind _returnvalue_2 (UserInterface|CreateWidget "/WM_InputManager_Plugin/WM_UMG/WM_InputManagerSmartMenu.WM_InputManagerSmartMenu_C"))
      (UserInterface|Viewport|AddtoViewport _returnvalue_2 0)
      (Class|WMInputManagerBase|SetNumberOfPlayers _returnvalue)
      (Class|WMInputManager|BeginUMG _returnvalue))
    (:then_1
      (Class|GameplayStatics|CreatePlayer -1)
      (Class|GameplayStatics|CreatePlayer -1)
      (Class|GameplayStatics|CreatePlayer -1)
      (Class|GameplayStatics|CreatePlayer -1))))

(event EventTick
  (params (DeltaSeconds :type Float%20%28single-precision%29))
  (bind _returnvalue (Class|GameModeBase|GetNumPlayers))
  (Class|WMInputManagerBase|SetNumberOfPlayers (Class|WMControllerFunctionLib|GetWMInputManager) _returnvalue))

(fn ConstructionScript)