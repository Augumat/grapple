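; Player input receiver that turns drift, dash, attack and grapple actions into per-frame input states, plus a mouse aim heading.
; Press and release events set buffer booleans, with presses also counted per frame.
; Each Tick finds BP_Player, derives yaw toward the mouse, then advances every input through a Rest/Pressed/Held state machine, keeping the previous frame's states.
; A toggleable debug overlay prints heading, states and press count.
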(event EventTick
  (params (DeltaSeconds :type Float%20%28single-precision%29))
  ;[0.6 0.6 1] Mouse Angle
  (bind _returnvalue (Actor|GetActorOfClass "/Game/BP_Player.BP_Player_C"))
  (Utilities|IsValid _returnvalue
    (:Is%20Valid
      (Variables|Aggregates|SetHeadingRotator (Math|Rotator|MakeRotator 0.0 0.0 (.Yaw (Math|Rotator|BreakRotator (Math|Rotator|FindLookatRotation (Transformation|GetActorLocation _returnvalue) (Utilities|GetMouseLocation))))))
      (CallFunction|TickforNextFrame))
    (:Is%20Not%20Valid
      (Development|PrintString "[ERROR] No BP_Player in level" true true "(R=1.000000,G=0.000000,B=0.000000,A=1.000000)"))))

(event Input|ActionEvents|InputActionSpecialAttack
  (params (Key :type Key%20Structure :default "None"))
  ;[1 0.6 0.6] Action Buttons
  (:Pressed
    (Utilities|ReceiveNewInputState (Variables|AsyncInputs|GetSpecialAttackState) :!label _label))
  (:Released
    (goto _label Released)))

(event Input|ActionEvents|InputActionSpoolGrapple
  (params (Key :type Key%20Structure :default "None"))
  ;[0.6 1 0.6] Movement Buttons
  (:Pressed
    (Utilities|ReceiveNewInputState (Variables|AsyncInputs|GetSpoolGrappleState) :!label _label))
  (:Released
    (goto _label Released)))

(event Input|ActionEvents|InputActionToggleDebugOverlay
  (params (Key :type Key%20Structure :default "None"))
  ;[0 0 0] Debug
  (:Pressed
    (bind _output_get (Variables|SyncInputs|SetDebugEnabled (not (Variables|SyncInputs|GetDebugEnabled))))
    (Development|PrintString (Utilities|String|Append "Set Debug = " (Utilities|String|ToString(Boolean) _output_get)) true true "(R=0.505208,G=0.002513,B=0.000000,A=1.000000)")))

(event Input|ActionEvents|InputActionNeutralAttack
  (params (Key :type Key%20Structure :default "None"))
  ;[1 0.6 0.6] Action Buttons
  (:Pressed
    (Utilities|ReceiveNewInputState (Variables|AsyncInputs|GetNeutralAttackState) :!label _label))
  (:Released
    (goto _label Released)))

(event Input|ActionEvents|InputActionDriftLeft
  (params (Key :type Key%20Structure :default "None"))
  ;[1 1 0.6] Drifting Buttons
  (:Pressed
    (Utilities|ReceiveNewInputState (Variables|AsyncInputs|GetDriftLeftState) :!label _label))
  (:Released
    (goto _label Released)))

(event Input|ActionEvents|InputActionDriftRight
  (params (Key :type Key%20Structure :default "None"))
  ;[1 1 0.6] Drifting Buttons
  (:Pressed
    (Utilities|ReceiveNewInputState (Variables|AsyncInputs|GetDriftRightState) :!label _label))
  (:Released
    (goto _label Released)))

(event Input|ActionEvents|InputActionDriftUp
  (params (Key :type Key%20Structure :default "None"))
  ;[1 1 0.6] Drifting Buttons
  (:Pressed
    (Utilities|ReceiveNewInputState (Variables|AsyncInputs|GetDriftUpState) :!label _label))
  (:Released
    (goto _label Released)))

(event Input|ActionEvents|InputActionDriftDown
  (params (Key :type Key%20Structure :default "None"))
  ;[1 1 0.6] Drifting Buttons
  (:Pressed
    (Utilities|ReceiveNewInputState (Variables|AsyncInputs|GetDriftDownState) :!label _label))
  (:Released
    (goto _label Released)))

(event Input|ActionEvents|InputActionDash
  (params (Key :type Key%20Structure :default "None"))
  ;[0.6 1 0.6] Movement Buttons
  (:Pressed
    (Utilities|ReceiveNewInputState (Variables|AsyncInputs|GetDashState) :!label _label))
  (:Released
    (goto _label Released)))

(event Input|ActionEvents|InputActionFireGrapple
  (params (Key :type Key%20Structure :default "None"))
  ;[0.6 1 0.6] Movement Buttons
  (:Pressed
    (Utilities|ReceiveNewInputState (Variables|AsyncInputs|GetFireGrappleState) :!label _label))
  (:Released
    (goto _label Released)))

(event Input|ActionEvents|InputActionPullGrapple
  (params (Key :type Key%20Structure :default "None"))
  ;[0.6 1 0.6] Movement Buttons
  (:Pressed
    (Utilities|ReceiveNewInputState (Variables|AsyncInputs|GetPullGrappleState) :!label _label))
  (:Released
    (goto _label Released)))

(fn ConstructionScript)

(fn TickforNextFrame
  (bind _self self)
  (Utilities|FlowControl|Sequence
    (:then_0
      ;[1 1 1] update and reset frameinputs
      (bind _newstatearray (CallFunction|HandleStateTransitions (Variables|Aggregates|GetCurrentFrameInputs) (Utilities|GetStateBuffer)))
      (Variables|Aggregates|SetPreviousFrameInputs (Variables|Aggregates|GetCurrentFrameInputs))
      (Variables|Aggregates|SetCurrentFrameInputs _newstatearray))
    (:then_1
      ;[1 1 1] update and reset input counter
      (Variables|Aggregates|SetCurrentFrameTotalInputs (Variables|Default|GetInputsThisFrameRunningTotal))
      (Variables|Default|SetInputsThisFrameRunningTotal 0))
    (:then_2
      ;[0 0 0] debug for input handling
      (if (Variables|SyncInputs|GetDebugEnabled)
        (Class|KismetSystemLibrary|FlushDebugStrings)
        (Development|PrintString (Utilities|String|ToString(Rotator) (Variables|Aggregates|GetHeadingRotator _self)) true true "(R=0.510306,G=0.805439,B=1.000000,A=1.000000)" 0.01)
        (for _array_element (Variables|Aggregates|GetCurrentFrameInputs _self)
          (LocalVariables|SetDebugArrayPrintString (Utilities|String|Append (LocalVariables|GetDebugArrayPrintString) " " (Utilities|String|EnumtoString _array_element))))
        (Development|PrintString (LocalVariables|GetDebugArrayPrintString) true true "(R=0.149130,G=0.453125,B=0.269927,A=1.000000)" 0.01)
        (Development|PrintString (Utilities|String|ToString(Integer) (Variables|Aggregates|GetCurrentFrameTotalInputs _self)) true true "(R=0.218750,G=1.000000,B=0.335363,A=1.000000)" 0.01)))))

(fn HandleStateTransitions
  (params (CurrentStateArray :type Array%20of%20ButtonInputState%20Enums :default "NewEnumerator0") (StateBuffer :type Array%20of%20Booleans))
  (for (_array_element _array_index) CurrentStateArray
    (bind _newstate (CallFunction|HandleStateTransition _array_element (Utilities|Array|Get(acopy) StateBuffer _array_index)))
    (Utilities|Array|SetArrayElem (LocalVariables|GetTempStateArray) _array_index _newstate true))
  (return (LocalVariables|GetTempStateArray)))

(fn HandleStateTransition
  (params (CurrentState :type ButtonInputState%20Enum :default "NewEnumerator0") (BufferState :type Boolean))
  (switch Utilities|FlowControl|Switch|SwitchonButtonInputState CurrentState
    (:NewEnumerator0
      (if BufferState
        (LocalVariables|SetTempState "NewEnumerator1")
        (else
          (LocalVariables|SetTempState "NewEnumerator0" :!label _label))))
    (:NewEnumerator1
      (if BufferState
        (LocalVariables|SetTempState "NewEnumerator2" :!label _label_2)
        (else
          (goto _label))))
    (:NewEnumerator2
      (if BufferState
        (goto _label_2)
        (else
          (goto _label)))))
  (return (LocalVariables|GetTempState)))